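; BP_BaseCharacter is a base character that handles health, a flashlight and the character creation screen at start.
; BeginPlay shows the CharacterCreation widget, activates Camcam instead of CameraComponent and disables input.
; AnyDamage subtracts from CurrentHealth; both it and Tick disable player input at zero or below.
; Tick hides the SpotLight when FlashlightOn is true or the battery is empty, otherwise shows it, so the flag reads inverted.
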(event EventBeginPlay
  (bind _returnvalue (UserInterface|CreateWidget "/Game/UI_Widget/CharacterCreation.CharacterCreation_C"))
  (UserInterface|Viewport|AddtoViewport _returnvalue 0)
  (Components|Activation|SetActive (Variables|Default|Getcamcam) true false)
  (Components|Activation|SetActive (Variables|Default|GetCameraComponent) false false)
  (Input|DisableInput 0))

(event Collision|EventActorBeginOverlap
  (params (OtherActor :type Actor%20Object%20Reference)))

(event EventTick
  (params (DeltaSeconds :type Float%20%28single-precision%29))
  (bind _spotlight (Variables|Default|GetSpotLight))
  (Utilities|FlowControl|Sequence
    (:then_0
      (if (<= (Variables|Default|GetCurrentHealth) 0.0)
        (Input|DisableInput (Game|GetPlayerController 0))))
    (:then_1
      (if (Variables|Default|GetFlashlightOn)
        (Rendering|SetVisibility _spotlight false false :!label _label)
        (elif (<= (Variables|Default|GetFlashlightBattery) 0.0)
          (goto _label)
          (else
            (Rendering|SetVisibility _spotlight true false)))))))

(event Game|Damage|EventAnyDamage
  (params (Damage :type Float%20%28single-precision%29) (DamageType :type Damage%20Type%20Object%20Reference) (InstigatedBy :type Controller%20Object%20Reference) (DamageCauser :type Actor%20Object%20Reference))
  (bind _output_get (Variables|Default|SetCurrentHealth (- (Variables|Default|GetCurrentHealth) Damage)))
  (Math|Float|CompareFloat _output_get 0.0
    (:==
      _)
    (:<
      _))
  (Input|DisableInput (Game|GetPlayerController 0)))

(fn ConstructionScript)