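; BP_FinishButton is an interactable button that ends the game in victory once the quota is reached.
; On interact it reads Quota from the BP_QuotaComputer in the level and compares it to a hardcoded target.
; On success it disables player input, shows the VictoryScreen widget with the cursor, and sets the cached character's health and oxygen very high.
; Below the target, it only prints the current quota.
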(event EventBeginPlay
  (bind _asbp_base_character (Utilities|Casting|CastToBP_BaseCharacter (Game|GetPlayerCharacter 0)))
  (Variables|Default|SetAs%20BP%20Base%20Character _asbp_base_character))

(event Collision|EventActorBeginOverlap
  (params (OtherActor :type Actor%20Object%20Reference)))

(event EventTick
  (params (DeltaSeconds :type Float%20%28single-precision%29)))

(event EventOnInteract
  (bind _as_bp_base_character (Variables|Default|GetAs%20BP%20Base%20Character))
  (bind _returnvalue (Actor|GetActorOfClass "/Game/Blueprints/BP_QuotaComputer.BP_QuotaComputer_C"))
  (if (>= (Variables|/Script/GAD2006Final_SHL.QuotaComputer|GetQuota _returnvalue) 350)
    (Variables|Default|SetIsTargetQuotaReached true)
    (Input|DisableInput (Game|Player|GetPlayerPawn 0) (Game|GetPlayerController 0))
    (bind _returnvalue_2 (UserInterface|CreateWidget "/Game/UI_Widget/VictoryScreen.VictoryScreen_C" (Game|GetPlayerController 0)))
    (UserInterface|Viewport|AddtoViewport _returnvalue_2 0)
    (Variables|/Script/GAD2006Final_SHL.BaseCharacter|SetCurrentHealth _as_bp_base_character 1e+03)
    (Variables|/Script/GAD2006Final_SHL.BaseCharacter|SetCurrentOxygen _as_bp_base_character 1e+03)
    (Variables|/Script/Engine.PlayerController|SetbShowMouseCursor (Game|GetPlayerController 0) true)
    (else
      (Development|PrintString (Utilities|String|ToString(Integer) (Variables|/Script/GAD2006Final_SHL.QuotaComputer|GetQuota _returnvalue))))))

(fn ConstructionScript)