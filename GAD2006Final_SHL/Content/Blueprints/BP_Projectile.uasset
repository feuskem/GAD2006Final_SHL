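; BP_Projectile is a short-lived projectile that damages BP_BaseCharacter actors it overlaps.
; An actor overlap destroys it when the other actor is tagged Duvar or TurretTarget.
; Its Sphere overlap destroys it if the Sphere itself carries Duvar; otherwise it damages characters with non-zero health and destroys itself.
; Non-character overlaps trigger delayed destruction, alongside a fixed lifespan set at BeginPlay.
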(event OnComponentBeginOverlap(Sphere)
  (params (OverlappedComponent :type Primitive%20Component%20Object%20Reference) (OtherActor :type Actor%20Object%20Reference) (OtherComp :type Primitive%20Component%20Object%20Reference) (OtherBodyIndex :type Integer) (bFromSweep :type Boolean) (SweepResult :type Hit%20Result%20Structure%20%28by%20ref%29))
  (if (Components|ComponentHasTag OverlappedComponent "Duvar")
    (Actor|DestroyActor)
    (else
      (bind _asbp_base_character (Utilities|Casting|CastToBP_BaseCharacter OtherActor)
        (:then
          (if (not (== (Variables|/Script/GAD2006Final_SHL.BaseCharacter|GetCurrentHealth _asbp_base_character) 0.0))
            (Game|Damage|ApplyDamage _asbp_base_character 1.0 0 0)
            (Actor|DestroyActor)))
        (:CastFailed
          (Utilities|FlowControl|Delay 5.0)
          (Actor|DestroyActor))))))

(event EventBeginPlay
  (Actor|SetLifeSpan 5.0))

(event Collision|EventActorBeginOverlap
  (params (OtherActor :type Actor%20Object%20Reference))
  (if (or (Actor|ActorHasTag OtherActor "Duvar") (Actor|ActorHasTag OtherActor "TurretTarget"))
    (Actor|DestroyActor)))

(event EventTick
  (params (DeltaSeconds :type Float%20%28single-precision%29)))

(fn ConstructionScript)