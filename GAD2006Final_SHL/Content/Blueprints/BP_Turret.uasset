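; BP_Turret is an automated turret that sweeps for targets and fires projectiles in bursts.
; Tick runs a Searching/Attacking state machine, swinging the poseable mesh's base bone back and forth while searching.
; PawnSensing turns the bone toward pawns tagged TurretTarget, stores their location and restarts a timer that returns to searching.
; Attacking launches BP_Projectile at that location with sound, using a flag and delays to pace shots and bursts.
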(event OnSeePawn(PawnSensing)
  (params (Pawn :type Pawn%20Object%20Reference))
  (bind _poseablemesh (Variables|Default|GetPoseableMesh))
  ;[1 1 1] On See Pawn
  (if (Actor|ActorHasTag Pawn "TurretTarget")
    (Variables|Default|SetTargetLocation (Transformation|GetActorLocation Pawn))
    (Variables|Default|SetTurretState "NewEnumerator1")
    (bind _returnvalue (Class|PoseableMeshComponent|GetBoneRotationbyName _poseablemesh "DEF_Base_002" "WorldSpace"))
    (Components|PoseableMesh|SetBoneRotationbyName _poseablemesh "DEF_Base_002" (Math|Rotator|MakeRotator (.roll _returnvalue) (.pitch _returnvalue) (- (.yaw (Math|Rotator|FindLookatRotation (Transformation|GetActorLocation) (Variables|Default|GetTargetLocation))) 1.8e+02)) "WorldSpace")
    (Utilities|Time|ClearandInvalidateTimerbyHandle (Variables|Default|GetReset%20Turret%20State%20Timer))
    (bind _returnvalue_2 (Utilities|Time|SetTimerbyEvent (delegate Custom|Reset%20Turret%20State) 1.0))
    (Variables|Default|SetReset%20Turret%20State%20Timer _returnvalue_2)))

(event Custom|Rotate%20Turret
  (bind _returnvalue (Utilities|Time|GetWorldDeltaSeconds))
  (bind _returnvalue_2 (* _returnvalue 5e+01))
  ;[1 1 1] Rotate Turret
  (bind _returnvalue_3 (Class|PoseableMeshComponent|GetBoneRotationbyName (Variables|Default|GetPoseableMesh) "DEF_Base_002" "ComponentSpace"))
  (Variables|Default|SetShould%20Turret%20Rotate%20Right (or (and (< (.Yaw (Math|Rotator|BreakRotator _returnvalue_3)) 7e+01) (Variables|Default|GetShould%20Turret%20Rotate%20Right)) (and (< (.Yaw (Math|Rotator|BreakRotator _returnvalue_3)) -7e+01) (not (Variables|Default|GetShould%20Turret%20Rotate%20Right)))))
  (Components|PoseableMesh|SetBoneRotationbyName (Variables|Default|GetPoseableMesh) "DEF_Base_002" (Math|Rotator|MakeRotator (.Roll (Math|Rotator|BreakRotator _returnvalue_3)) (.Pitch (Math|Rotator|BreakRotator _returnvalue_3)) (Math|Float|SelectFloat (+ (.Yaw (Math|Rotator|BreakRotator _returnvalue_3)) _returnvalue_2) (- (.Yaw (Math|Rotator|BreakRotator _returnvalue_3)) _returnvalue_2) (Variables|Default|GetShould%20Turret%20Rotate%20Right))) "ComponentSpace"))

(event Custom|Turret%20Attack
  (bind _arrow (Variables|Default|GetArrow))
  (bind _targetlocation (Variables|Default|GetTargetLocation))
  (bind _returnvalue (Transformation|GetWorldLocation _arrow))
  (bind _returnvalue_2 (Math|Vector|GetUnitDirection(Vector) _returnvalue _targetlocation))
  ;[1 1 1] Turret Attacking Logic
  (if (not (Variables|Default|GetIs%20Attacking))
    (Variables|Default|SetIs%20Attacking true)
    (bind _returnvalue_3 (Game|SpawnActorfromClass "/Game/Blueprints/BP_Projectile.BP_Projectile_C" (Math|Transform|MakeTransform (+ _returnvalue (* _returnvalue_2 6e+01)) "0, 0, 0" "1.000000,1.000000,1.000000") "Undefined" 0 0))
    (Audio|PlaySound2D "/Game/UI_Widget/Projectilesfx.Projectilesfx" 1.0 1.0 0.0 0 0)
    (Physics|SetPhysicsLinearVelocity (Variables|/Game/Blueprints/BP_Projectile.BP_Projectile_C|GetSphere _returnvalue_3) (* _returnvalue_2 3e+03) false "None")
    (Utilities|FlowControl|Delay (Variables|Default|GetDelay%20Between%20Attacks))
    (bind _result (Math|Integer|IncrementInt (Variables|Default|GetNumber%20Of%20Attacks%20Done))
      (:%20%20
        (if (>= _result (Variables|Default|GetAttack%20Frequency))
          (Variables|Default|SetNumber%20Of%20Attacks%20Done 0)
          (Utilities|FlowControl|Delay (Variables|Default|GetDelay%20Between%20Multiple%20Attacks)))
        (Variables|Default|SetIs%20Attacking false)))))

(event Custom|Reset%20Turret%20State
  ;[1 1 1] On See Pawn
  (Variables|Default|SetTurretState "NewEnumerator0"))

(event EventBeginPlay)

(event Collision|EventActorBeginOverlap
  (params (OtherActor :type Actor%20Object%20Reference)))

(event EventTick
  (params (DeltaSeconds :type Float%20%28single-precision%29))
  ;[1 1 1] Event Tick
  (switch Utilities|FlowControl|Switch|SwitchonTurret_State (Variables|Default|GetTurretState)
    (:NewEnumerator0
      (CallFunction|RotateTurret))
    (:NewEnumerator1
      (CallFunction|TurretAttack))))

(fn ConstructionScript)